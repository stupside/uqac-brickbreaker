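; BP_GridSpawner is an actor that spawns a 2D grid of actors of a configurable class, positioned relative to the player.
; On BeginPlay it sets the grid center at the first player pawn's location, shifted along Y by an offset plus sector size times the Y count.
; A 2DGridExecutionMacro walks the cells, and the spawner creates one actor at each cell center with itself as owner.
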(event EventBeginPlay
  (bind _poly_center (Utilities|2DGridExecutionMacro (Variables|Spawn|GetSector%20Size) (+ (Math|Vector|MakeVector 0.0 (Variables|Spawn|GetOffset) 0.0) (Transformation|GetActorLocation (Game|Player|GetPlayerPawn 0)) (* (* (Variables|Spawn|GetSector%20Size) (Variables|Spawn|GetSize%20Y)) "0.000000,1.000000,0.000000")) (Variables|Spawn|GetSize%20X) (Variables|Spawn|GetSize%20Y))
    (:Per%20Poly%20Execution
      (Game|SpawnActorfromClass (Variables|Spawn|GetClass) (Math|Conversions|ToTransform(Vector) _poly_center) "Undefined" self 0))))

(fn ConstructionScript)